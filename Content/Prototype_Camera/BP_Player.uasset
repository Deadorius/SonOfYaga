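; BP_Player is the player Blueprint for a camera prototype, handling movement, facing and a dialogue test.
; Enhanced Input IA_Movement adds movement along forward and right vectors derived only from control yaw.
; A Lookat event rotates the actor toward a target using its X and Y coordinates.
; DialogueTest creates the TESTDIALOG widget with TEST dialogue, adds it to the viewport and shows the mouse cursor.
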(event `DialogueTest`
  (bind _returnvalue (`|CreateWidget` "/Game/Prototype_Camera/TESTDIALOG.TESTDIALOG_C" null "/Game/TEST.TEST" self null))
  (`UserWidget.AddToViewport` _returnvalue 0)
  (set `PlayerController.bShowMouseCursor` true (`GameplayStatics.GetPlayerController` 0)))

(event `EnhancedInput|/Game/Prototype_Camera/IA_Movement`
  (params (ActionValue :type "Vector2D Structure") (ElapsedSeconds :type "Float (double-precision)") (TriggeredSeconds :type "Float (double-precision)") (InputAction :type "InputAction Object Reference" :default "/Game/Prototype_Camera/IA_Movement.IA_Movement"))
  (bind (_returnvalue_roll _returnvalue_pitch _returnvalue_yaw) (`KismetMathLibrary.BreakRotator` (`self.GetControlRotation`)))
  (bind _returnvalue (`KismetMathLibrary.MakeRotator` 0.0 0.0 _returnvalue_yaw))
  (:`Triggered`
    (`|ExecutionSequence`
      (:`then_0`
        (`self.AddMovementInput` (`KismetMathLibrary.GetForwardVector` _returnvalue) ActionValue_Y))
      (:`then_1`
        (`self.AddMovementInput` (`KismetMathLibrary.GetRightVector` _returnvalue) ActionValue_X)))))

(event `/Game/Prototype_Camera/BPI_PlayerInterface.Look At`
  (params (Target :type "Vector Structure"))
  (bind (_returnvalue_x _returnvalue_y) (`KismetMathLibrary.BreakVector` (`self.K2_GetActorLocation`)))
  (`self.K2_SetActorRotation` (`KismetMathLibrary.FindLookAtRotation` (`KismetMathLibrary.MakeVector` _returnvalue_x _returnvalue_y) (`KismetMathLibrary.MakeVector` Target_X Target_Y))))

(fn `UserConstructionScript`)